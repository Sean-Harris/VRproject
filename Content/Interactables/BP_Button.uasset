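; BP_Button is an interactable with separate ON and OFF buttons that broadcasts ONPressed and OFFPressed events.
; Each Tick measures the distance between each button component and its constraint to detect a press.
; A press fires once past the far threshold and re-arms only when the button returns near its constraint, giving hysteresis against repeated triggers.
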(event EventBeginPlay)

(event EventTick
  (params (DeltaSeconds :type Float%20%28single-precision%29))
  (bind _offbutton (Variables|Default|GetOFFButton))
  (bind _onbutton (Variables|Default|GetONButton))
  (bind _offconstraint (Variables|Default|GetOFFConstraint))
  (bind _onconstraint (Variables|Default|GetONConstraint))
  (bind _returnvalue (Transformation|GetWorldLocation _onconstraint))
  (bind _returnvalue_2 (Transformation|GetWorldLocation _offbutton))
  (bind _returnvalue_3 (Transformation|GetWorldLocation _offconstraint))
  (bind _returnvalue_4 (Transformation|GetWorldLocation _onbutton))
  (bind _returnvalue_5 (Math|Vector|Distance(Vector) _returnvalue_2 _returnvalue_3))
  (bind _returnvalue_6 (Math|Vector|Distance(Vector) _returnvalue_4 _returnvalue))
  (Utilities|FlowControl|Sequence
    (:then_0
      (if (> _returnvalue_5 4.2)
        (if (not (Variables|Default|GetOFFBeingPressed))
          (Default|CallOFFPressed)
          (Variables|Default|SetOFFBeingPressed true))
        (elif (< _returnvalue_5 1.0)
          (Variables|Default|SetOFFBeingPressed false))))
    (:then_1
      (if (> _returnvalue_6 4.2)
        (if (not (Variables|Default|GetONBeingPressed))
          (Default|CallONPressed)
          (Variables|Default|SetONBeingPressed true))
        (elif (< _returnvalue_6 1.0)
          (Variables|Default|SetONBeingPressed false))))))

(fn ConstructionScript)