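; Non-Euclidean cube object that builds six portal faces, each paired with its own capture portal.
; On BeginPlay it spawns a BP_NonEuclidianPlane at each face component (Bottom, Top, Front, Back, Right, Left) and attaches it snapped to that component.
; For each face it spawns a BP_NonEuclidianPlaneCaptureActor and passes it the viewing plane, the matching capture portal and a shared render target resolution.
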(event EventBeginPlay
  (bind _renderwidth (Variables|Default|GetRenderWidth))
  (bind _renderheight (Variables|Default|GetRenderHeight))
  (Utilities|FlowControl|Sequence
    (:then_0
      (bind _noneuclidianplane (CallFunction|SpawnandAttachCubeFace (Variables|Default|GetBottom)))
      (bind _output_get (Variables|Default|SetBottomPlane _noneuclidianplane))
      (CallFunction|SpawnandConfigureCaptureActor _output_get (Variables|Default|GetBottomCapture) _renderwidth _renderheight))
    (:then_1
      (bind _noneuclidianplane_2 (CallFunction|SpawnandAttachCubeFace (Variables|Default|GetTop)))
      (bind _output_get_2 (Variables|Default|SetTopPlane _noneuclidianplane_2))
      (CallFunction|SpawnandConfigureCaptureActor _output_get_2 (Variables|Default|GetTopCapture) _renderwidth _renderheight))
    (:then_2
      (bind _noneuclidianplane_3 (CallFunction|SpawnandAttachCubeFace (Variables|Default|GetFront)))
      (bind _output_get_3 (Variables|Default|SetFrontPlane _noneuclidianplane_3))
      (CallFunction|SpawnandConfigureCaptureActor _output_get_3 (Variables|Default|GetFrontCapture) _renderwidth _renderheight))
    (:then_3
      (bind _noneuclidianplane_4 (CallFunction|SpawnandAttachCubeFace (Variables|Default|GetBack)))
      (bind _output_get_4 (Variables|Default|SetBackPlane _noneuclidianplane_4))
      (CallFunction|SpawnandConfigureCaptureActor _output_get_4 (Variables|Default|GetBackCapture) _renderwidth _renderheight))
    (:then_4
      (bind _noneuclidianplane_5 (CallFunction|SpawnandAttachCubeFace (Variables|Default|GetRight)))
      (bind _output_get_5 (Variables|Default|SetRightPlane _noneuclidianplane_5))
      (CallFunction|SpawnandConfigureCaptureActor _output_get_5 (Variables|Default|GetRightCapture) _renderwidth _renderheight))
    (:then_5
      (bind _noneuclidianplane_6 (CallFunction|SpawnandAttachCubeFace (Variables|Default|GetLeft)))
      (bind _output_get_6 (Variables|Default|SetLeftPlane _noneuclidianplane_6))
      (CallFunction|SpawnandConfigureCaptureActor _output_get_6 (Variables|Default|GetLeftCapture) _renderwidth _renderheight))))

(event EventTick
  (params (DeltaSeconds :type Float%20%28single-precision%29)))

(fn ConstructionScript)

(fn SpawnandAttachCubeFace
  (params (SceneComp :type Scene%20Component%20Object%20Reference))
  (bind _returnvalue (Game|SpawnActorfromClass "/Game/Tehtävä2/BP_NonEuclidianPlane.BP_NonEuclidianPlane_C" (Transformation|GetWorldTransform SceneComp) "AlwaysSpawn" 0 0))
  (Transformation|AttachComponentToComponent _returnvalue SceneComp "None" "SnapToTarget" "SnapToTarget" "SnapToTarget" true)
  (return _returnvalue))

(fn SpawnandConfigureCaptureActor
  (params (ViewingPortal :type BP%20Non%20Euclidian%20Plane%20Object%20Reference) (CapturePortal :type Actor%20Object%20Reference) (RenderTargetWidth :type Integer) (RenderTargetHeight :type Integer))
  (bind _returnvalue (Game|SpawnActorfromClass "/Game/Tehtävä2/BP_NonEuclidianPlaneCaptureActor.BP_NonEuclidianPlaneCaptureActor_C" (Math|Transform|MakeTransform "0, 0, 0" "0, 0, 0" "1.000000,1.000000,1.000000") "AlwaysSpawn" 0 0))
  (Variables|/Game/Tehtävä2/BP_NonEuclidianPlaneCaptureActor.BP_NonEuclidianPlaneCaptureActor_C|SetViewingPortal _returnvalue ViewingPortal)
  (Variables|/Game/Tehtävä2/BP_NonEuclidianPlaneCaptureActor.BP_NonEuclidianPlaneCaptureActor_C|SetCapturePortal _returnvalue CapturePortal)
  (Variables|/Game/Tehtävä2/BP_NonEuclidianPlaneCaptureActor.BP_NonEuclidianPlaneCaptureActor_C|SetRenderTargetWidth _returnvalue RenderTargetWidth)
  (Variables|/Game/Tehtävä2/BP_NonEuclidianPlaneCaptureActor.BP_NonEuclidianPlaneCaptureActor_C|SetRenderTargetHeight _returnvalue RenderTargetHeight))