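; Portal renderer that shows the view through a paired capture portal on the viewing portal's plane for the VR player.
; Each tick it mirrors the player camera into the capture portal's space and clips captures at that portal.
; Custom projections scale each render target to the portal's on-screen bounds, skipping capture when out of view.
; A dynamic material receives the textures and view-projection columns, with a right-eye capture set up under stereo rendering.
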(event EventBeginPlay
  (bind _asbp_vrcharacter (Utilities|Casting|CastToBP_VRCharacter (Game|Player|GetPlayerPawn 0)))
  (Variables|Default|SetPlayerPawn _asbp_vrcharacter)
  (Variables|Default|SetPlayerCamera (Variables|/Game/Player/BP_VRCharacter.BP_VRCharacter_C|GetCamera (Variables|Default|GetPlayerPawn)))
  ;[1 1 1] Create a material using the render target(s) as its texture and apply it to the portal plane
  (bind _returnvalue (Rendering|Material|CreateDynamicMaterialInstance "/Game/PortalSampleMaterial.PortalSampleMaterial" "None" "None" :!class /Script/Engine.KismetMaterialLibrary))
  (Variables|Default|SetPortalMID _returnvalue)
  (Rendering|Material|SetMaterial (Variables|/Game/PortalBP.PortalBP_C|GetPortalPlane (Variables|Default|GetViewingPortal)) 0 (Variables|Default|GetPortalMID))
  (bind _rendertarget (CallFunction|SetupCaptureComponent (Variables|Default|GetCaptureComponentLeftEye)))
  (Rendering|Material|SetTextureParameterValue (Variables|Default|GetPortalMID) "PortalTextureLeftEye" _rendertarget))

(event EventTick
  (params (DeltaSeconds :type Float%20%28single-precision%29))
  (bind _capturecomponentlefteye (Variables|Default|GetCaptureComponentLeftEye))
  (bind _capturecomponentlefteye_2 (Variables|Default|GetCaptureComponentLeftEye))
  (bind _scenecomponent (Variables|Default|GetSceneComponent))
  (bind _capturecomponentrighteye (Variables|Default|GetCaptureComponentRightEye))
  (bind _returnvalue (Transformation|GetWorldTransform _scenecomponent))
  (bind (_outrotation _outposition) (Class|PortalCaptureActor|AdjustLeftEyePose (.rotation _returnvalue) (.location _returnvalue)))
  (bind (_outrotation_2 _outposition_2) (Class|PortalCaptureActor|AdjustRightEyePose (.rotation _returnvalue) (.location _returnvalue)))
  (CallFunction|CheckStereoActivation)
  ;[1 1 1] Compute the portal camera's position
  (Transformation|SetWorldLocation (Variables|Default|GetSceneComponent) (Math|Transform|TransformLocation (Transformation|GetActorTransform (Variables|Default|GetCapturePortal)) (* (Math|Transform|InverseTransformLocation (Transformation|GetActorTransform (Variables|Default|GetViewingPortal)) (Transformation|GetWorldLocation (Variables|Default|GetPlayerCamera))) "-1.000000,-1.000000,1.000000")) false false)
  (Transformation|SetWorldRotation (Variables|Default|GetSceneComponent) (Math|Transform|TransformRotation (Transformation|GetActorTransform (Variables|Default|GetCapturePortal)) (Math|Rotator|CombineRotators (Math|Transform|InverseTransformRotation (Transformation|GetActorTransform (Variables|Default|GetViewingPortal)) (Transformation|GetWorldRotation (Variables|Default|GetPlayerCamera))) "0,180.000000, 0")) false false)
  (if (Class|PortalCaptureActor|IsRenderingStereo)
    ;[1 1 1 0] Stereoscopic Rendering
    (Transformation|SetWorldTransform (Variables|Default|GetCaptureComponentLeftEye) (Math|Transform|MakeTransform _outposition _outrotation (.scale _returnvalue)) false false)
    (Transformation|SetWorldTransform (Variables|Default|GetCaptureComponentRightEye) (Math|Transform|MakeTransform _outposition_2 _outrotation_2 (.scale _returnvalue)) false false)
    (bind _desiredview (Class|CameraComponent|GetCameraView (Variables|Default|GetPlayerCamera) DeltaSeconds))
    ;;[1 1 1 0] Left Eye
    (CallFunction|UpdateClipPlane _capturecomponentlefteye_2)
    (CallFunction|UpdateCaptureState _capturecomponentlefteye_2 (Variables|/Game/PortalBP.PortalBP_C|GetPortalPlane (Variables|Default|GetViewingPortal)) (.ViewMatrix (Class|GameplayStatics|GetViewProjectionMatrix (Class|PortalCaptureActor|AdjustLeftEyeViewInfo _desiredview))) (Class|PortalCaptureActor|GetLeftEyeProjection) "LeftViewProjection_Col0" "LeftViewProjection_Col1" "LeftViewProjection_Col3")
    ;;[1 1 1 0 16] Right Eye
    (CallFunction|UpdateClipPlane _capturecomponentrighteye)
    (CallFunction|UpdateCaptureState _capturecomponentrighteye (Variables|/Game/PortalBP.PortalBP_C|GetPortalPlane (Variables|Default|GetViewingPortal)) (.ViewMatrix (Class|GameplayStatics|GetViewProjectionMatrix (Class|PortalCaptureActor|AdjustRightEyeViewInfo _desiredview))) (Class|PortalCaptureActor|GetRightEyeProjection) "RightViewProjection_Col0" "RightViewProjection_Col1" "RightViewProjection_Col3")
    (else
      ;[1 1 1 0 16] Monoscopic Rendering
      (bind _desiredview_2 (Class|CameraComponent|GetCameraView (Variables|Default|GetPlayerCamera) DeltaSeconds))
      (CallFunction|UpdateClipPlane _capturecomponentlefteye)
      (CallFunction|UpdateCaptureState _capturecomponentlefteye (Variables|/Game/PortalBP.PortalBP_C|GetPortalPlane (Variables|Default|GetViewingPortal)) (.ViewMatrix (Class|GameplayStatics|GetViewProjectionMatrix _desiredview_2)) (.ProjectionMatrix (Class|GameplayStatics|GetViewProjectionMatrix _desiredview_2)) "LeftViewProjection_Col0" "LeftViewProjection_Col1" "LeftViewProjection_Col3"))))

(event Collision|EventActorBeginOverlap
  (params (OtherActor :type Actor%20Object%20Reference)))

(fn ConstructionScript)

(fn GetScaledViewProjection
  (params (Mesh :type Static%20Mesh%20Component%20Object%20Reference) (ViewProjection :type Matrix%20Structure) (Projection :type Matrix%20Structure))
  (bind (_min _max) (Components|StaticMesh|GetLocalBounds Mesh))
  (bind _returnvalue (Transformation|GetWorldTransform Mesh))
  (bind _returnvalue_2 (Math|Transform|ToMatrix(Transform) _returnvalue))
  (bind _returnvalue_3 (* _returnvalue_2 ViewProjection))
  (bind (_minpointndc _maxpointndc _isinview) (Class|PortalCaptureActor|ClipPortalScreenBounds _min _max _returnvalue_3))
  (LocalVariables|SetScale (/ (Math|Vector2D|MakeVector2D 2.0 2.0) (- _maxpointndc _minpointndc)))
  (LocalVariables|SetOffset (- (Math|Vector2D|MakeVector2D -1.0 -1.0) (* (LocalVariables|GetScale) _minpointndc)))
  (return (* ViewProjection (Math|Transform|ToMatrix(Transform) (Math|Transform|MakeTransform (Math|Conversions|ToVector(Vector2D) (LocalVariables|GetOffset)) "0, 0, 0" (Math|Conversions|ToVector(Vector2D) (LocalVariables|GetScale) 1.0)))) (* Projection (Math|Transform|ToMatrix(Transform) (Math|Transform|MakeTransform (Math|Conversions|ToVector(Vector2D) (LocalVariables|GetOffset)) "0, 0, 0" (Math|Conversions|ToVector(Vector2D) (LocalVariables|GetScale) 1.0)))) _isinview))

(fn SetupCaptureComponent
  (params (Capture%20Component :type Scene%20Capture%20Component%202D%20Object%20Reference))
  (Components|Activation|SetActive Capture%20Component true false)
  (bind _returnvalue (Rendering|CreateRenderTarget2D (Variables|Default|GetRenderTargetWidth) (Variables|Default|GetRenderTargetHeight) "RTF_RGBA8"))
  (bind _output_get (Variables|/Script/Engine.SceneCaptureComponent2D|SetTextureTarget Capture%20Component _returnvalue))
  (Variables|/Script/Engine.SceneCaptureComponent2D|SetbUseCustomProjectionMatrix Capture%20Component true)
  (return _output_get))

(fn UpdateClipPlane
  (params (CaptureComponent :type Scene%20Capture%20Component%202D%20Object%20Reference))
  (bind _captureportal (Variables|Default|GetCapturePortal))
  (bind _returnvalue (Transformation|GetActorForwardVector _captureportal))
  (Variables|/Script/Engine.SceneCaptureComponent2D|SetClipPlaneNormal CaptureComponent _returnvalue)
  (Variables|/Script/Engine.SceneCaptureComponent2D|SetClipPlaneBase CaptureComponent (+ (Transformation|GetActorLocation _captureportal) (* _returnvalue 0.01))))

(fn CheckStereoActivation
  (if (Class|PortalCaptureActor|IsRenderingStereo)
    (if (not (Variables|Default|GetHasActivatedStereo))
      (bind _rendertarget (CallFunction|SetupCaptureComponent (Variables|Default|GetCaptureComponentRightEye)))
      (Rendering|Material|SetTextureParameterValue (Variables|Default|GetPortalMID) "PortalTextureRightEye" _rendertarget)
      (Variables|Default|SetHasActivatedStereo true))
    (else
      (Components|Activation|SetActive (Variables|Default|GetCaptureComponentRightEye) false false))))

(fn UpdateCaptureState
  (params (CaptureComponent :type Scene%20Capture%20Component%202D%20Object%20Reference) (PortalMesh :type Static%20Mesh%20Component%20Object%20Reference) (View :type Matrix%20Structure) (Projection :type Matrix%20Structure) (ViewProjectionCol0Name :type Name) (ViewProjectionCol1Name :type Name) (ViewProjectionCol3Name :type Name))
  (bind _returnvalue (* View Projection))
  (bind _portalmid (Variables|Default|GetPortalMID))
  (bind (_scaledviewprojection _scaledprojection _isinview) (CallFunction|GetScaledViewProjection PortalMesh _returnvalue Projection))
  (bind _returnvalue_2 (Class|KismetMathLibrary|MatrixGetTransposed _scaledviewprojection))
  (if _isinview
    (Variables|/Script/Engine.SceneCaptureComponent2D|SetCustomProjectionMatrix CaptureComponent _scaledprojection)
    (Rendering|Material|SetVectorParameterValue _portalmid ViewProjectionCol0Name (Utilities|PlanetoLinearColor (.xplane _returnvalue_2)) :!class /Script/Engine.MaterialInstanceDynamic)
    (Rendering|Material|SetVectorParameterValue _portalmid ViewProjectionCol1Name (Utilities|PlanetoLinearColor (.yplane _returnvalue_2)) :!class /Script/Engine.MaterialInstanceDynamic)
    (Rendering|Material|SetVectorParameterValue _portalmid ViewProjectionCol3Name (Utilities|PlanetoLinearColor (.wplane _returnvalue_2)) :!class /Script/Engine.MaterialInstanceDynamic)
    (Rendering|SceneCapture|CaptureScene CaptureComponent :!class /Script/Engine.SceneCaptureComponent2D)))